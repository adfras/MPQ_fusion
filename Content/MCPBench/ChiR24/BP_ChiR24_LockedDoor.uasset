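; BP_ChiR24_LockedDoor is a door actor that opens on overlap only once its key has been granted.
; The MCP_GrantKey event sets HasKey, which ActorBeginOverlap checks without filtering the overlapping actor.
; With the key, a DoOnce gate sets IsOpen, prints a message and eases the root component to a fixed location with MoveComponentTo.
; Without the key, it only prints locked messages.
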(event `MCP_GrantKey`
  (set `self.HasKey` true))

(event `self.ReceiveActorBeginOverlap`
  (params (OtherActor :type "Actor Object Reference"))
  (if (`self.HasKey`)
    (`|DoOnceMultiInput`
      (:`A Out`
        (set `self.IsOpen` true)
        (`KismetSystemLibrary.PrintString` "door opened")
        (`KismetSystemLibrary.MoveComponentTo` (`self.K2_GetRootComponent`) (620.0 0.0 260.0) (struct) true true 1.25)))
    (else
      (`KismetSystemLibrary.PrintString` "Need key")
      (`KismetSystemLibrary.PrintString` "door locked"))))

(fn `UserConstructionScript`)
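; Test sequence-console actor that, on any actor overlap, runs a timed gate-and-bridge show guarded by an IsActive flag.
; Chained MoveComponentTo calls press the switch, raise the gate and extend three bridge segments, turning pillars green and brightening a light.
; After a delay it retracts everything in reverse, restores materials and light, then clears the flag to re-arm.
; Print strings log each stage.
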(event `self.ReceiveActorBeginOverlap`
  (params (OtherActor :type "Actor Object Reference"))
  (bind _activationswitch (`self.ActivationSwitch`))
  (bind _sequencelight (`self.SequenceLight`))
  (bind _gate (`self.Gate`))
  (bind _bridgeplatform1 (`self.BridgePlatform1`))
  (bind _bridgeplatform2 (`self.BridgePlatform2`))
  (bind _bridgeplatform3 (`self.BridgePlatform3`))
  (bind _statuspillar1 (`self.StatusPillar1`))
  (bind _statuspillar2 (`self.StatusPillar2`))
  (bind _statuspillar3 (`self.StatusPillar3`))
  (if (not (`self.IsActive`))
    (set `self.IsActive` true)
    (`KismetSystemLibrary.PrintString` "SEQ START")
    (`PrimitiveComponent.SetMaterial` _activationswitch 0 "/Game/TestingKit/Automation/AgentTests/M_Codex_Seq_Green.M_Codex_Seq_Green")
    (`KismetSystemLibrary.MoveComponentTo` _activationswitch (0.0 0.0 4.0) (struct) false false 0.25)
    (`LightComponent.SetIntensity` _sequencelight 7000.0)
    (`KismetSystemLibrary.MoveComponentTo` _gate (185.0 0.0 220.0) (struct) false false 0.45)
    (`KismetSystemLibrary.MoveComponentTo` _bridgeplatform1 (360.0 0.0 16.0) (struct) false false 0.45)
    (`KismetSystemLibrary.PrintString` "SEGMENT 1 EXTENDED")
    (`PrimitiveComponent.SetMaterial` _statuspillar1 0 "/Game/TestingKit/Automation/AgentTests/M_Codex_Seq_Green.M_Codex_Seq_Green")
    (`KismetSystemLibrary.MoveComponentTo` _bridgeplatform2 (520.0 0.0 16.0) (struct) false false 0.45)
    (`KismetSystemLibrary.PrintString` "SEGMENT 2 EXTENDED")
    (`PrimitiveComponent.SetMaterial` _statuspillar2 0 "/Game/TestingKit/Automation/AgentTests/M_Codex_Seq_Green.M_Codex_Seq_Green")
    (`KismetSystemLibrary.MoveComponentTo` _bridgeplatform3 (680.0 0.0 16.0) (struct) false false 0.45)
    (`KismetSystemLibrary.PrintString` "SEGMENT 3 EXTENDED")
    (`PrimitiveComponent.SetMaterial` _statuspillar3 0 "/Game/TestingKit/Automation/AgentTests/M_Codex_Seq_Green.M_Codex_Seq_Green")
    (`KismetSystemLibrary.Delay` 4.0)
    (`KismetSystemLibrary.PrintString` "SEQ RESET")
    (`KismetSystemLibrary.MoveComponentTo` _bridgeplatform3 (680.0 -115.0 16.0) (struct) false false 0.3)
    (`KismetSystemLibrary.MoveComponentTo` _bridgeplatform2 (520.0 -115.0 16.0) (struct) false false 0.3)
    (`KismetSystemLibrary.MoveComponentTo` _bridgeplatform1 (360.0 -115.0 16.0) (struct) false false 0.3)
    (`KismetSystemLibrary.MoveComponentTo` _gate (185.0 0.0 80.0) (struct) false false 0.35)
    (`PrimitiveComponent.SetMaterial` _activationswitch 0 "/Game/TestingKit/Automation/AgentTests/M_Codex_Seq_Red.M_Codex_Seq_Red")
    (`KismetSystemLibrary.MoveComponentTo` _activationswitch (0.0 0.0 18.0) (struct) false false 0.25)
    (`LightComponent.SetIntensity` _sequencelight 600.0)
    (`PrimitiveComponent.SetMaterial` _statuspillar1 0 "/Game/TestingKit/Automation/AgentTests/M_Codex_Seq_Dark.M_Codex_Seq_Dark")
    (`PrimitiveComponent.SetMaterial` _statuspillar2 0 "/Game/TestingKit/Automation/AgentTests/M_Codex_Seq_Dark.M_Codex_Seq_Dark")
    (`PrimitiveComponent.SetMaterial` _statuspillar3 0 "/Game/TestingKit/Automation/AgentTests/M_Codex_Seq_Dark.M_Codex_Seq_Dark")
    (set `self.IsActive` false)
    (`KismetSystemLibrary.PrintString` "SEQ COMPLETE")))

(fn `UserConstructionScript`)
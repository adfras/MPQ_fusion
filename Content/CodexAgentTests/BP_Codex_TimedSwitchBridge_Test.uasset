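; Test actor for a timed switch bridge: any actor overlap presses the pad, raises a gate post and extends three bridge segments, then resets after a delay.
; One latent chain of MoveComponentTo and Delay nodes staggers the segments and retracts them in reverse order.
; Switch material and pad light intensity signal the state, and an IsActive flag ignores overlaps until the reset completes.
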(event `self.ReceiveActorBeginOverlap`
  (params (OtherActor :type "Actor Object Reference"))
  (bind _switchmesh (`self.SwitchMesh`))
  (bind _gatepost (`self.GatePost`))
  (bind _bridgesegment1 (`self.BridgeSegment1`))
  (bind _bridgesegment2 (`self.BridgeSegment2`))
  (bind _bridgesegment3 (`self.BridgeSegment3`))
  (bind _padlight (`self.PadLight`))
  (if (not (`self.IsActive`))
    (set `self.IsActive` true)
    (`KismetSystemLibrary.PrintString` "Timed bridge activated")
    (`PrimitiveComponent.SetMaterial` _switchmesh 0 "/Game/TestingKit/Automation/AgentTests/M_Codex_TimedSwitch_Green.M_Codex_TimedSwitch_Green")
    (`LightComponent.SetIntensity` _padlight 6500.0)
    (`KismetSystemLibrary.MoveComponentTo` _switchmesh (0.0 0.0 0.0) (struct) true true 0.25)
    (`KismetSystemLibrary.MoveComponentTo` _gatepost (240.0 0.0 220.0) (struct) true true 0.65)
    (`KismetSystemLibrary.Delay` 0.18)
    (`KismetSystemLibrary.MoveComponentTo` _bridgesegment1 (620.0 0.0 12.0) (struct) true true 0.45)
    (`KismetSystemLibrary.Delay` 0.18)
    (`KismetSystemLibrary.MoveComponentTo` _bridgesegment2 (830.0 0.0 12.0) (struct) true true 0.45)
    (`KismetSystemLibrary.Delay` 0.18)
    (`KismetSystemLibrary.MoveComponentTo` _bridgesegment3 (1040.0 0.0 12.0) (struct) true true 0.45)
    (`KismetSystemLibrary.Delay` 5.0)
    (`KismetSystemLibrary.PrintString` "Bridge resetting")
    (`KismetSystemLibrary.MoveComponentTo` _bridgesegment3 (550.0 0.0 12.0) (struct) true true 0.45)
    (`KismetSystemLibrary.MoveComponentTo` _bridgesegment2 (470.0 0.0 12.0) (struct) true true 0.45)
    (`KismetSystemLibrary.MoveComponentTo` _bridgesegment1 (390.0 0.0 12.0) (struct) true true 0.45)
    (`KismetSystemLibrary.MoveComponentTo` _gatepost (240.0 0.0 75.0) (struct) true true 0.65)
    (`KismetSystemLibrary.MoveComponentTo` _switchmesh (0.0 0.0 6.0) (struct) true true 0.25)
    (`PrimitiveComponent.SetMaterial` _switchmesh 0 "/Game/TestingKit/Automation/AgentTests/M_Codex_TimedSwitch_Red.M_Codex_TimedSwitch_Red")
    (`LightComponent.SetIntensity` _padlight 650.0)
    (set `self.IsActive` false)))

(fn `UserConstructionScript`)